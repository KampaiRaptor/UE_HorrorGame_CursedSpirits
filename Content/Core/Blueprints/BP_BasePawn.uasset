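; BP_BasePawn is a player pawn that turns Enhanced Input into camera look, movement animation and an attack.
; On BeginPlay it adds the base mapping context for player 0 and caches the mesh's MainCharacterAnimBP.
; Look input drives controller yaw and pitch, and left click plays the attack montage.
; Movement input only sets the anim Blueprint's forward and sideways values, zeroed on release, with no movement applied in this graph.
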(event Input|EnhancedActionEvents|EnhancedInputActionIA_Look
  (params (ActionValue :type Vector%202D%20Structure) (ElapsedSeconds :type Float%20%28double-precision%29) (TriggeredSeconds :type Float%20%28double-precision%29) (InputAction :type Input%20Action%20Object%20Reference :default "/Game/Core/Input/IA_Look.IA_Look"))
  (Pawn|Input|AddControllerYawInput (.x ActionValue))
  (Pawn|Input|AddControllerPitchInput (.y ActionValue)))

(event Input|EnhancedActionEvents|EnhancedInputActionIA_Movement
  (params (ActionValue :type Vector%202D%20Structure) (ElapsedSeconds :type Float%20%28double-precision%29) (TriggeredSeconds :type Float%20%28double-precision%29) (InputAction :type Input%20Action%20Object%20Reference :default "/Game/Core/Input/IA_Movement.IA_Movement"))
  (bind _maincharacteranimbp (Variables|Default|GetMainCharacterAnimBP))
  (bind _maincharacteranimbp_2 (Variables|Default|GetMainCharacterAnimBP))
  (:Triggered
    (Variables|/Game/Art/Characters/MainCharacterAnimBP.MainCharacterAnimBP_C|SetAnim_MovingSideway _maincharacteranimbp_2 (.x ActionValue))
    (Variables|/Game/Art/Characters/MainCharacterAnimBP.MainCharacterAnimBP_C|SetAnim_MovingForward _maincharacteranimbp_2 (.y ActionValue)))
  (:Completed
    (Variables|/Game/Art/Characters/MainCharacterAnimBP.MainCharacterAnimBP_C|SetAnim_MovingSideway _maincharacteranimbp 0.0)
    (Variables|/Game/Art/Characters/MainCharacterAnimBP.MainCharacterAnimBP_C|SetAnim_MovingForward _maincharacteranimbp 0.0)))

(event Input|EnhancedActionEvents|EnhancedInputActionIA_LeftClick
  (params (ActionValue :type Float%20%28double-precision%29) (ElapsedSeconds :type Float%20%28double-precision%29) (TriggeredSeconds :type Float%20%28double-precision%29) (InputAction :type Input%20Action%20Object%20Reference :default "/Game/Core/Input/IA_LeftClick.IA_LeftClick"))
  (:Started
    (Animation|Montage|PlayMontage (Variables|Character|GetMesh) "/Game/Art/Characters/Animations/PlayerAttackMontage.PlayerAttackMontage")))

(event EventBeginPlay
  (bind _returnvalue (Game|GetPlayerController 0))
  (bind _returnvalue_2 (PlayerController|LocalPlayerSubsystems|GetEnhancedInputLocalPlayerSubsystem _returnvalue))
  (Utilities|IsValid _returnvalue_2
    (:Is%20Valid
      (Input|AddMappingContext _returnvalue_2 "/Game/Core/Input/PM_BaseMappingContext.PM_BaseMappingContext" 0 "(bIgnoreAllPressedKeysUntilRelease=True,bForceImmediately=False,bNotifyUserSettings=False)")
      (bind _asmain_character_anim_bp (Utilities|Casting|CastToMainCharacterAnimBP (Components|SkeletalMesh|GetAnimInstance (Variables|Character|GetMesh))))
      (Variables|Default|SetMainCharacterAnimBP _asmain_character_anim_bp))))

(fn ConstructionScript)