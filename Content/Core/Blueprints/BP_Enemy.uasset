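; Spirit enemy Actor that homes in on the player and drains their health on contact.
; Tick rotates and offsets it toward the player without sweep or delta-time scaling; sphere overlap halts it and sends drain messages each frame until the player moves out of range.
; Niagara and mesh color switch between green and red with drain state.
; Any damage notifies the player pawn, ragdolls the mesh and destroys the actor after a delay.
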(event OnComponentBeginOverlap(Sphere1)
  (params (OverlappedComponent :type Primitive%20Component%20Object%20Reference) (OtherActor :type Actor%20Object%20Reference) (OtherComp :type Primitive%20Component%20Object%20Reference) (OtherBodyIndex :type Integer) (bFromSweep :type Boolean) (SweepResult :type Hit%20Result%20Structure%20%28by%20ref%29))
  (bind _returnvalue (Math|Color|MakeColor 5e+01 0.0 0.0))
  (if (and (== OtherActor (Game|Player|GetPlayerPawn 0)) (== (Variables|Default|GetbDrainingPlayer) false))
    (Variables|Default|SetbDrainingPlayer true)
    (Niagara|SetNiagaraVariable(LinearColor) (Variables|Default|GetNiagara) "ParticleColor" _returnvalue)
    (Rendering|Material|SetVectorParameterValueonMaterials (Variables|Default|GetSkeletalMesh) "Color" (/ (Math|Conversions|ToVector(LinearColor) _returnvalue) 5e+01))))

(event EventBeginPlay
  (Components|Animation|PlayAnimation (Variables|Default|GetSkeletalMesh) (.OutItem (Utilities|Array|Random (Utilities|Array|MakeArray "/Game/Art/Characters/Animations/ZombieWalk_UE.ZombieWalk_UE" "/Game/Art/Characters/Animations/Walking_1__UE.Walking_1__UE" "/Game/Art/Characters/Animations/Walking_UE.Walking_UE"))) true)
  (Utilities|FlowControl|Delay (Math|Random|RandomFloatinRange 1.0 3.0) :!label _label)
  (bind _spiritsound (Variables|Default|GetSpiritSound)
    (:then
      (Components|Activation|Activate _spiritsound true)
      (goto _label))
    (:else)))

(event EventTick
  (params (DeltaSeconds :type Float%20%28single-precision%29))
  (bind _returnvalue (Game|Player|GetPlayerPawn 0))
  (bind _returnvalue_2 (Math|Color|MakeColor 0.0 5e+01 0.0))
  (bind _skeletalmesh (Variables|Default|GetSkeletalMesh))
  (bind _returnvalue_3 (Transformation|GetActorLocation _returnvalue))
  (bind _returnvalue_4 (Transformation|GetWorldLocation _skeletalmesh))
  (bind _returnvalue_5 (Math|Conversions|ToVector(LinearColor) _returnvalue_2))
  (bind _returnvalue_6 (- _returnvalue_3 "0.000000,0.000000,70.000000"))
  (bind _returnvalue_7 (/ _returnvalue_5 5e+01))
  (bind _returnvalue_8 (Math|Rotator|FindLookatRotation _returnvalue_4 _returnvalue_6))
  (if (Variables|Default|GetbDrainingPlayer)
    (Class|DamageInterface|DIDrainHealth(Message) (Game|Player|GetPlayerPawn 0))
    (if (> (Math|Vector|Distance(Vector) (Transformation|GetWorldLocation (Variables|Default|GetSkeletalMesh)) (Transformation|GetActorLocation (Game|Player|GetPlayerPawn 0))) 3e+02)
      (Variables|Default|SetbDrainingPlayer false)
      (Niagara|SetNiagaraVariable(LinearColor) (Variables|Default|GetNiagara) "ParticleColor" _returnvalue_2)
      (Rendering|Material|SetVectorParameterValueonMaterials (Variables|Default|GetSkeletalMesh) "Color" _returnvalue_7)
      (Development|PrintString (Utilities|String|ToString(Vector) _returnvalue_7)))
    (else
      (Transformation|SetActorRotation _returnvalue_8)
      (Transformation|AddActorWorldOffset (* (Math|Vector|GetForwardVector _returnvalue_8) (Variables|Default|GetSpeed))))))

(event Game|Damage|EventAnyDamage
  (params (Damage :type Float%20%28single-precision%29) (DamageType :type Damage%20Type%20Object%20Reference) (InstigatedBy :type Controller%20Object%20Reference) (DamageCauser :type Actor%20Object%20Reference))
  (bind _returnvalue (Math|Color|MakeColor 0.0 5e+01 0.0))
  (bind _skeletalmesh (Variables|Default|GetSkeletalMesh))
  (Class|DamageInterface|DISpiritKilled(Message) (Game|Player|GetPlayerPawn 0))
  (Components|DestroyComponent (Variables|Default|GetSphere1))
  (Actor|Tick|SetActorTickEnabled false)
  (Collision|SetCollisionEnabled _skeletalmesh "QueryAndPhysics")
  (Class|SkeletalMeshComponent|SetAllBodiesSimulatePhysics _skeletalmesh true)
  (Audio|PlaySoundatLocation "/Game/Art/Sounds/esm_ancient_game_dark_magic_gust_spell_2_fantasy_tonal_accent_hit_stab.esm_ancient_game_dark_magic_gust_spell_2_fantasy_tonal_accent_hit_stab" (Transformation|GetActorLocation) "0, 0, 0" 1.0 1.0 0.0 "/Game/Art/Sounds/Att_Setting.Att_Setting" 0 0 0)
  (Niagara|SetNiagaraVariable(LinearColor) (Variables|Default|GetNiagara) "ParticleColor" _returnvalue)
  (Rendering|Material|SetVectorParameterValueonMaterials (Variables|Default|GetSkeletalMesh) "Color" (/ (Math|Conversions|ToVector(LinearColor) _returnvalue) 5e+01))
  (Utilities|FlowControl|Delay 1e+01)
  (Actor|DestroyActor))

(fn ConstructionScript)