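; BP_Altar is an altar that lights its fire the first time the player pawn overlaps its sphere.
; A DoOnce gate plays the LightUpAnim timeline at half speed, ramping the fire effect's ash spawn rate, fire spawn rate and light intensity up from zero.
; When the animation finishes, it calls CheckAltars on the BP_BasePawn found in the level.
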(event OnComponentBeginOverlap(Sphere)
  (params (OverlappedComponent :type Primitive%20Component%20Object%20Reference) (OtherActor :type Actor%20Object%20Reference) (OtherComp :type Primitive%20Component%20Object%20Reference) (OtherBodyIndex :type Integer) (bFromSweep :type Boolean) (SweepResult :type Hit%20Result%20Structure%20%28by%20ref%29))
  (if (== OtherActor (Game|Player|GetPlayerPawn 0))
    (CallFunction|LightUp)))

(event Custom|LightUp
  (Utilities|FlowControl|DoOnce false
    (:Completed
      (Components|Timeline|SetPlayRate (Variables|Default|GetLightUpAnim) 0.5)
      (bind _float (Timeline|LightUpAnim PlayFromStart)
        (:Update
          (Niagara|SetNiagaraVariable(Float) (Variables|Default|GetP_Fire_03) "Ashes_SpawnRate" (Math|Float|Lerp 0.0 15.0 _float))
          (Niagara|SetNiagaraVariable(Float) (Variables|Default|GetP_Fire_03) "Fire_SpawnRate" (Math|Float|Lerp 0.0 15.0 _float))
          (Niagara|SetNiagaraVariable(Float) (Variables|Default|GetP_Fire_03) "LightIntensity" (Math|Float|Lerp 0.0 1.0 _float)))
        (:Finished
          (bind _returnvalue (Actor|GetActorOfClass "/Game/Core/Blueprints/BP_BasePawn.BP_BasePawn_C"))
          (Default|CheckAltars _returnvalue))))))

(fn ConstructionScript)